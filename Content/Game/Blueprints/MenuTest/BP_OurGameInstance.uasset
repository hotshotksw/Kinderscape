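; Game instance that handles multiplayer hosting and joining through Advanced Sessions nodes.
; CreateSession creates a session with the UseLAN flag, then opens L_Jayden as a listen server.
; JoinAdvanceSession searches client-hosted servers and joins a random result, with no check for an empty list.
; SetLAN toggles UseLAN, which the search does not use, and failures only print debug strings.
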(event Custom|CreateSession
  (|AdvancedSession 0 (Game|GetPlayerController 0) 100 0 (Variables|Default|GetUse%20LAN) true false true true true false false false true false true
    (:OnSuccess
      (Game|OpenLevel(byObjectReference) "/Game/Game/Levels/L_Jayden.L_Jayden" true "listen"))
    (:OnFailure
      (Development|PrintString "Failed to create session :("))))

(event Custom|JoinAdvanceSession
  (bind _results (|FindSessionsAdvanced (Game|GetPlayerController 0) 1000 false "ClientServersOnly" 0 false false false true)
    (:OnSuccess
      (|JoinSession (Game|GetPlayerController 0) (Utilities|Array|Get(acopy) _results (Math|Random|RandomIntegerinRange 0 (- (Utilities|Array|Length _results) 1)))
        (:OnSuccess
          (Development|PrintString "Joining session :)"))
        (:OnFailure
          (Development|PrintString "Failed to join session :("))))
    (:OnFailure
      (Development|PrintString "Failed to find session :("))))

(event Custom|SetLAN
  (if (Variables|Default|GetUse%20LAN)
    (Variables|Default|SetUse%20LAN false)
    (else
      (Variables|Default|SetUse%20LAN true))))