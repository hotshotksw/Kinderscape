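; BP_Book is a book prop that plays a hit sound when it overlaps another BP_Book.
; The construction script sets its static mesh from Block.
; Begin overlap passes a DoOnce before the cast, so any actor can use up the gate, and the sound plays at the other book's location.
; The gate resets one second after an overlap with another book ends.
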(event EventBeginPlay)

(event Collision|EventActorBeginOverlap
  (params (OtherActor :type Actor%20Object%20Reference))
  (Utilities|FlowControl|DoOnce false
    (:Completed
      (bind _asbp_book (Utilities|Casting|CastToBP_Book OtherActor))
      (Audio|PlaySoundatLocation "/Game/Game/Audio/block_hit.block_hit" (Transformation|GetActorLocation _asbp_book) "0, 0, 0" 1.0 1.0 0.0 0 0 0 0))))

(event EventTick
  (params (DeltaSeconds :type Float%20%28single-precision%29)))

(event Collision|EventActorEndOverlap
  (params (OtherActor :type Actor%20Object%20Reference))
  (Utilities|Casting|CastToBP_Book OtherActor)
  (Utilities|FlowControl|Delay 1.0)
  (Utilities|FlowControl|DoOnce false) ; enters at Reset
)

(fn ConstructionScript
  (Components|StaticMesh|SetStaticMesh (Variables|Default|GetStaticMesh) (Variables|Default|GetBlock)))